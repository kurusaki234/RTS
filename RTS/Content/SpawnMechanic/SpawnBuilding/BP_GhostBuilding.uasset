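; Placement preview actor that shows a building's mesh snapped to a grid at the cursor's world position.
; ConstructBuilding briefly spawns the chosen building to read its display mesh and construction proxy, resets the ghost, then destroys that temporary actor.
; OnSpawn stores this data and opens a Tick gate for snapped movement, while KillGhost clears it and closes the gate.
; Both set the controller's BuildModeActive to true, including KillGhost.
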(event `OnSpawn`
  (params (DisplayMesh :type "StaticMesh Object Reference") (BuildingClass :type "/Game/MyFolder/SpawnBuilding/BP_BuildingMaster Class Reference") (ConstructionProxy :type "/Game/MyFolder/SpawnBuilding/BP_ConstructionProxy Class Reference"))
  ;[1 1 1] OnSpawn
  (if (not (`self.IsActive`))
    (set `self.BuildingClass` BuildingClass)
    (set `self.ConstructionProxy` ConstructionProxy)
    (set `self.DisplayMesh` DisplayMesh)
    (set `self.IsActive` true)
    (set `/Game/MyFolder/BP_CameraPawnController.BuildModeActive` true (`self.ControllerRef`))
    (`StaticMeshComponent.SetStaticMesh` (`self.GhostBuilding_Mesh`) (`self.DisplayMesh`))
    (`self.OpenTickGate`)))

(event `KillGhost`
  ;[1 1 1] Kill Ghost
  (set `self.BuildingClass` null)
  (set `self.ConstructionProxy` null)
  (`self.CloseTickGate`)
  (set `self.DisplayMesh` null)
  (set `self.IsActive` false)
  (set `/Game/MyFolder/BP_CameraPawnController.BuildModeActive` true (`self.ControllerRef`))
  (`StaticMeshComponent.SetStaticMesh` (`self.GhostBuilding_Mesh`) (`self.DisplayMesh`)))

(event `/Game/MyFolder/BP_MyInterface.ConstructBuilding`
  (params (MainBuilding :type "/Game/MyFolder/SpawnBuilding/BP_BuildingMaster Class Reference"))
  (bind _returnvalue (`|SpawnActorFromClass` MainBuilding (`KismetMathLibrary.MakeTransform` (0.0 0.0 0.0)) "Undefined" "OverrideRootScale" null (`self.ControllerRef`)))
  (`|ExecutionSequence`
    (:`then_0`
      (bind _asbp_building_master (castclass `/Game/MyFolder/SpawnBuilding/BP_BuildingMaster` MainBuilding))
      (`self.KillGhost`)
      (`self.OnSpawn` (`/Game/MyFolder/SpawnBuilding/BP_BuildingMaster.DisplayMesh` _returnvalue) _asbp_building_master (`/Game/MyFolder/SpawnBuilding/BP_BuildingMaster.ConstructionProxy` _returnvalue)))
    (:`then_1`
      (`self.K2_DestroyActor` _returnvalue))))

(event `self.ReceiveTick`
  (params (DeltaSeconds :type "Float (single-precision)"))
  (`/Engine/EditorBlueprintResources/StandardMacros.Gate` true :!label _label
    (:`Exit`
      (`self.K2_SetActorLocation` self (`self.SetGripSnapVector`) false false))))

(event `OpenTickGate`
  (goto _label :!via `Open`))

(event `CloseTickGate`
  (goto _label :!via `Close`))

(fn `SetGripSnapVector`
  (returns (GridSnap :type "Vector Structure"))
  (bind (_cursorworldposition_x _cursorworldposition_y _cursorworldposition_z) (`KismetMathLibrary.BreakVector` (`self.CursorWorldPosition`)))
  (bind _gridsize (`self.GridSize`))
  (return (`KismetMathLibrary.MakeVector` (`/Game/MyFolder/BP_MyFunctionLibrary.GridSnap` _cursorworldposition_x _gridsize) (`/Game/MyFolder/BP_MyFunctionLibrary.GridSnap` _cursorworldposition_y _gridsize) (`/Game/MyFolder/BP_MyFunctionLibrary.GridSnap` _cursorworldposition_z _gridsize))))

(fn `UserConstructionScript`)