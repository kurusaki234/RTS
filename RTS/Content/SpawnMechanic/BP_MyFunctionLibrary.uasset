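; Blueprint function library in the SpawnMechanic folder with helpers for cursor-based world positioning and grid snapping.
; SetCursorWorldPosition deprojects the mouse through the given controller, line traces up to SightDistance on a custom trace channel and returns the hit location when an actor is hit.
; GridSnap rounds a single axis value to the nearest multiple of GridSize by adding half a cell before flooring.
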(fn `GridSnap`
  (params (Axis :type "Float (double-precision)") (GridSize :type Integer))
  (returns (AxisOut :type "Float (double-precision)"))
  (return (`KismetMathLibrary.Conv_IntToDouble` (* (`KismetMathLibrary.FFloor` (/ (+ Axis (`KismetMathLibrary.Conv_IntToDouble` (/ GridSize 2))) (`KismetMathLibrary.Conv_IntToDouble` GridSize))) GridSize))))

(fn `SetCursorWorldPosition`
  (params (Controller :type "/Game/MyFolder/BP_CameraPawnController Object Reference") (SightDistance :type "Float (double-precision)"))
  (returns (Location :type "Vector Structure"))
  (bind (_worldlocation _worlddirection) (`PlayerController.DeprojectMousePositionToWorld` Controller))
  (bind _outhit (`KismetSystemLibrary.LineTraceSingle` null _worldlocation (+ _worldlocation (* _worlddirection SightDistance)) "TraceTypeQuery3"))
  (bind (_bblockinghit _binitialoverlap _time _location _impactpoint _normal _impactnormal _physmat _hitactor) (`GameplayStatics.BreakHitResult` _outhit))
  (if (!= _hitactor null)
    (return _location)))