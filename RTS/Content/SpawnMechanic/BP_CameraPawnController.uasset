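; Player controller for a top-down building camera that drives BP_CameraPawn and hosts build-mode placement.
; BeginPlay caches the pawn, spawns the construction manager and ghost building, and creates the UI.
; Axis input, screen-edge scrolling, gated mouse rotation and clamped spring-arm zoom move the camera, with axis speed scaling by zoom.
; In build mode, Tick feeds the cursor's world position to the ghost, and Deselect kills it.
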(event `self.ReceiveTick`
  (params (DeltaSeconds :type "Float (single-precision)"))
  (if (`self.BuildModeActive`)
    (if (!= (`self.GhostBuildingRef`) null)
      (set `/Game/MyFolder/SpawnBuilding/BP_GhostBuilding.CursorWorldPosition` (`/Game/MyFolder/BP_MyFunctionLibrary.SetCursorWorldPosition` self (`self.SetSightDistance`)) (`self.GhostBuildingRef`)))))

(event `InputAxis|MoveForward`
  (params (AxisValue :type "Float (single-precision)"))
  ;[1 1 1] Movement X
  (if (not (`self.DisableCameraNav`))
    (`self.K2_SetActorTransform` (`self.CameraPawnRef`) (`self.MovementX` AxisValue (`self.MovementSpeedCalculation`) (`self.FastMoveMultiplier`) (`self.CameraPawnRef`)) false false)))

(event `self.ReceiveBeginPlay`
  (bind _returnvalue (`KismetMathLibrary.MakeTransform` (0.0 0.0 0.0)))
  ;[1 1 1] Begin_Play
  (`|ExecutionSequence`
    (:`then_0`
      (`self.RefCast`))
    (:`then_1`
      (bind _returnvalue_2 (`|SpawnActorFromClass` "/Game/MyFolder/SpawnBuilding/BP_ConstructionManager.BP_ConstructionManager_C" _returnvalue "AlwaysSpawn" "OverrideRootScale"))
      (set `self.ConstructionManagerRef` _returnvalue_2))
    (:`then_2`
      (bind _returnvalue_3 (`|SpawnActorFromClass` "/Game/MyFolder/SpawnBuilding/BP_GhostBuilding.BP_GhostBuilding_C" _returnvalue "AlwaysSpawn" "OverrideRootScale" null self))
      (set `self.GhostBuildingRef` _returnvalue_3))
    (:`then_3`
      (`WidgetBlueprintLibrary.SetInputMode_GameAndUIEx` self null "LockOnCapture")
      (bind _returnvalue_4 (`|CreateWidget` "/Game/MyFolder/BP_MyUI.BP_MyUI_C" null self (`self.GhostBuildingRef`)))
      (`UserWidget.AddToViewport` _returnvalue_4 0))))

(event `InputAction|Deselect`
  (params (Key :type "Key Structure" :default "AnyKey"))
  (:`Pressed`
    (if (`self.BuildModeActive`)
      (`/Game/MyFolder/SpawnBuilding/BP_GhostBuilding.KillGhost` (`self.GhostBuildingRef`))
      (set `self.BuildModeActive` false))))

(event `InputAxis|MoveRight`
  (params (AxisValue :type "Float (single-precision)"))
  ;[1 1 1] Movement Y
  (if (not (`self.DisableCameraNav`))
    (`self.K2_SetActorTransform` (`self.CameraPawnRef`) (`KismetMathLibrary.MakeTransform` (`KismetMathLibrary.MakeVector` (.x (.location (`self.MovementY` AxisValue (`self.MovementSpeedCalculation`) (`self.FastMoveMultiplier`) (`self.CameraPawnRef`)))) (.y (.location (`self.MovementY` AxisValue (`self.MovementSpeedCalculation`) (`self.FastMoveMultiplier`) (`self.CameraPawnRef`)))) 100.0) (.rotation (`self.MovementY` AxisValue (`self.MovementSpeedCalculation`) (`self.FastMoveMultiplier`) (`self.CameraPawnRef`))) (.scale (`self.MovementY` AxisValue (`self.MovementSpeedCalculation`) (`self.FastMoveMultiplier`) (`self.CameraPawnRef`)))) false false)))

(event `InputAxisKey|MouseX`
  (params (AxisValue :type "Float (single-precision)"))
  ;[1 1 1] Pan X
  (`/Engine/EditorBlueprintResources/StandardMacros.Gate` true :!label _label
    (:`Exit`
      (`self.K2_SetActorRotation` (`self.CameraPawnRef`) (`KismetMathLibrary.MakeRotator` (.roll (`self.K2_GetActorRotation` (`self.CameraPawnRef`))) (.pitch (`self.K2_GetActorRotation` (`self.CameraPawnRef`))) (+ (.yaw (`self.K2_GetActorRotation` (`self.CameraPawnRef`))) (* (`self.PanSensitivity`) AxisValue))) false))))

(event `InputAction|Pan`
  (params (Key :type "Key Structure" :default "AnyKey"))
  ;[1 1 1] Pan X
  (:`Pressed`
    (set `self.DisableCameraNav` true)
    (goto _label :!via `Open`))
  (:`Released`
    (set `self.DisableCameraNav` false)
    (goto _label :!via `Close`)))

(event `InputAction|PanReset`
  (params (Key :type "Key Structure" :default "AnyKey"))
  (bind _camerapawnref (`self.CameraPawnRef`))
  ;[1 1 1] PanReset
  (:`Pressed`
    (`self.K2_SetActorRotation` _camerapawnref (`KismetMathLibrary.MakeRotator` (.roll (`self.K2_GetActorRotation` _camerapawnref)) 0.0 (.yaw (`self.K2_GetActorRotation` _camerapawnref))) false)))

(event `InputAxisKey|MouseY`
  (params (AxisValue :type "Float (single-precision)"))
  ;[1 1 1] Pan Y
  (`/Engine/EditorBlueprintResources/StandardMacros.Gate` true :!label _label_2
    (:`Exit`
      (`self.K2_SetActorRotation` (`self.CameraPawnRef`) (`KismetMathLibrary.MakeRotator` (.roll (`self.K2_GetActorRotation` (`self.CameraPawnRef`))) (`KismetMathLibrary.FClamp` (+ (.pitch (`self.K2_GetActorRotation` (`self.CameraPawnRef`))) (* (`self.PanSensitivity`) AxisValue)) -15.0 45.0) (.yaw (`self.K2_GetActorRotation` (`self.CameraPawnRef`)))) false))))

(event `InputAction|Pan`
  (params (Key :type "Key Structure" :default "AnyKey"))
  ;[1 1 1] Pan Y
  (:`Pressed`
    (set `self.DisableCameraNav` true)
    (goto _label_2 :!via `Open`))
  (:`Released`
    (set `self.DisableCameraNav` false)
    (goto _label_2 :!via `Close`)))

(event `InputAction|ZoomIn`
  (params (Key :type "Key Structure" :default "AnyKey"))
  (bind _springarm (`/Game/MyFolder/BP_CameraPawn.SpringArm` (`self.CameraPawnRef`)))
  ;[1 1 1] Zoom In/Out
  (:`Pressed`
    (set `SpringArmComponent.TargetArmLength` (`KismetMathLibrary.FClamp` (- (`SpringArmComponent.TargetArmLength` _springarm) (`self.ZoomSensitivity`)) 500.0 (`self.MaxArmDistance`)) _springarm)))

(event `InputAxisKey|MouseX`
  (params (AxisValue :type "Float (single-precision)"))
  ;[1 1 1] Edge Movement
  (if (not (`self.DisableCameraNav`))
    (bind (_deltaxspeed _deltayspeed) (`self.ScreenEdgeMovement` :!label _label_3))
    (`self.K2_AddActorLocalOffset` (`self.CameraPawnRef`) (`KismetMathLibrary.MakeVector` _deltaxspeed _deltayspeed) true false)))

(event `InputAction|ZoomOut`
  (params (Key :type "Key Structure" :default "AnyKey"))
  (bind _springarm (`/Game/MyFolder/BP_CameraPawn.SpringArm` (`self.CameraPawnRef`)))
  ;[1 1 1] Zoom In/Out
  (:`Pressed`
    (set `SpringArmComponent.TargetArmLength` (`KismetMathLibrary.FClamp` (+ (`SpringArmComponent.TargetArmLength` _springarm) (`self.ZoomSensitivity`)) 500.0 (`self.MaxArmDistance`)) _springarm)))

(event `InputAxisKey|MouseY`
  (params (AxisValue :type "Float (single-precision)"))
  ;[1 1 1] Edge Movement
  (if (not (`self.DisableCameraNav`))
    (goto _label_3 :!via `MouseY`)))

(fn `MovementSpeedCalculation`
  (returns (MoveSensitivity :type "Float (double-precision)"))
  (return (`KismetMathLibrary.FClamp` (/ (`SpringArmComponent.TargetArmLength` (`/Game/MyFolder/BP_CameraPawn.SpringArm` (`self.CameraPawnRef`))) 100.0) 5.0 20.0)))

(fn `SetSightDistance`
  (returns (SightDistance :type "Float (double-precision)"))
  (return (+ (`self.SightDistance`) (`SpringArmComponent.TargetArmLength` (`/Game/MyFolder/BP_CameraPawn.SpringArm` (`self.CameraPawnRef`))))))

(fn `UserConstructionScript`)